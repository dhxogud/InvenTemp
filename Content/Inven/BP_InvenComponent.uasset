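; Inventory component that holds item slots in an array and supports adding, removing and swapping items.
; On BeginPlay it creates ten slots filled with the "Empty" row from DT_Item, which serves as the empty-slot marker.
; AddItem copies a DT_Item row into the first empty slot without checking IsFull, and RemoveItem restores the Empty row.
; Every add, remove or swap prints all slots for debugging.
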(event EventBeginPlay
  (CallFunction|CreateInvenSlots 10))

(fn AddItem
  (params (RowName :type Name))
  (if (!= RowName "Empty")
    (bind _returnvalue (Utilities|GetDataTableRow "/Game/Inven/Item/DT_Item.DT_Item" RowName)
      (:then
        (bind _slotindex (CallFunction|FindEmptySlot))
        (Utilities|Array|SetArrayElem (Variables|Default|GetSlots) _slotindex (Utilities|Struct|MakeST_ItemSlot _slotindex _returnvalue))
        (CallFunction|PrintAllSlot)))))

(fn RemoveItem
  (params (Index :type Integer))
  (CallFunction|SetEmptySlot Index)
  (CallFunction|PrintAllSlot))

(fn SwapItem
  (params (FirstIndex :type Integer) (SecondIndex :type Integer))
  (Utilities|Array|Swap (Variables|Default|GetSlots) FirstIndex SecondIndex)
  (CallFunction|PrintAllSlot))

(fn CreateInvenSlots
  (params (Count :type Integer))
  (for _index (range 0 (- Count 1))
    (bind _returnvalue (Utilities|GetDataTableRow "/Game/Inven/Item/DT_Item.DT_Item" "Empty")
      (:then
        (Utilities|Array|Add (Variables|Default|GetSlots) (Utilities|Struct|MakeST_ItemSlot _index _returnvalue))))))

(fn IsEmptySlot
  (params (Index :type Integer))
  (return (Utilities|Enum|Equal(Enum) (.name (.ItemData (Utilities|Struct|BreakST_ItemSlot (Utilities|Array|Get(acopy) (Variables|Default|GetSlots) Index)))) "Empty")))

(fn SetEmptySlot
  (params (Index :type Integer))
  (bind _returnvalue (Utilities|GetDataTableRow "/Game/Inven/Item/DT_Item.DT_Item" "Empty")
    (:then
      (Utilities|Struct|SetmembersinST_ItemSlot (Utilities|Array|Get(acopy) (Variables|Default|GetSlots) Index) _returnvalue))))

(fn FindEmptySlot
  (for (_ _array_index) (Variables|Default|GetSlots)
    (if (CallFunction|IsEmptySlot _array_index)
      (return _array_index false)))
  (return -1 true))

(fn PrintAllSlot
  (for _array_element (Variables|Default|GetSlots)
    (Development|PrintString (Utilities|String|Append "Index : " (Utilities|String|ToString(Integer) (.Index (Utilities|Struct|BreakST_ItemSlot _array_element))) ", Name : " (.name (.ItemData (Utilities|Struct|BreakST_ItemSlot _array_element)))) true true "(R=0.000000,G=0.660000,B=1.000000,A=1.000000)" 1e+01)))